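; Door actor that opens and closes when hit, provided the referenced inventory holds at least one item.
; The Hit event checks only the Inventory length on KeyVarReference, so any item counts as a key.
; DoorOpen2 toggles the actor between two absolute rotations, snapping instantly with no interpolation.
; Debug strings print on both outcomes, including a closed message when the inventory is empty.
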(event `InputAction|Interact`)

(event `self.ReceiveHit`
  (params (MyComp :type "PrimitiveComponent Object Reference") (Other :type "Actor Object Reference") (OtherComp :type "PrimitiveComponent Object Reference") (bSelfMoved :type Boolean) (HitLocation :type "Object.Vector Structure") (HitNormal :type "Object.Vector Structure") (NormalImpulse :type "Object.Vector Structure") (Hit :type "EngineTypes.HitResult Structure (by ref)"))
  (if (>= (`KismetArrayLibrary.Array_Length` (`MyFPSCharacter.Inventory` (`self.KeyVarReference`))) 1)
    (`KismetSystemLibrary.PrintString` "Hello")
    (if (`self.doorOpen2`)
      (`self.SetActorRotation` (struct :`Yaw` 180.0))
      (set `self.doorOpen2` false)
      (else
        (`self.SetActorRotation` (struct :`Yaw` 90.0))
        (set `self.doorOpen2` true)))
    (else
      (`KismetSystemLibrary.PrintString` "Door closed"))))

(fn `UserConstructionScript`)